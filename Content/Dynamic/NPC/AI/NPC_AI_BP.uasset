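; AI controller for guard NPCs that drives a possessed TP_Character through patrol and combat.
; On begin play it sets up the PatrolData blackboard and runs the GuardBehavior tree.
; Perception updates store sensed actors lacking the "Enemy" tag under EnemyKey, clearing it when sensing fails.
; Each tick it sets the character's Aiming and Shooting flags whenever the controller has a valid focus actor.
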(event `self.ReceiveBeginPlay`
  (bind _blackboardcomponent (`self.UseBlackboard` "/Game/Dynamic/NPC/AI/PatrolData.PatrolData"))
  (`self.RunBehaviorTree` "/Game/Dynamic/NPC/AI/GuardBehavior.GuardBehavior")
  (set `self.BlackboardComp` _blackboardcomponent))

(event `self.ReceiveTick`
  (params (DeltaSeconds :type "Float (single-precision)"))
  (bind _astp_character (cast `/Game/Dynamic/NPC/Behavior/TP_Character` (`self.K2_GetPawn`)))
  (bind _output_get (set `/Game/Dynamic/NPC/Behavior/TP_Character.Aiming` (`KismetSystemLibrary.IsValid` (`self.GetFocusActor`)) _astp_character))
  (set `/Game/Dynamic/NPC/Behavior/TP_Character.Shooting` _output_get _astp_character))

(event `self.AIPerception.OnTargetPerceptionUpdated`
  (params (Actor :type "Actor Object Reference") (Stimulus :type "AIStimulus Structure"))
  (bind _blackboardcomp (`self.BlackboardComp`))
  (bind _enemykey (`self.EnemyKey`))
  (if (`self.ActorHasTag` Actor "Enemy")
    _
    (elif (`.bSuccessfullySensed` (break `AIStimulus` Stimulus))
      (`AIPerceptionSystem.GetSenseClassForStimulus` Stimulus)
      (`BlackboardComponent.SetValueAsObject` _blackboardcomp _enemykey Actor)
      (else
        (`BlackboardComponent.ClearValue` _blackboardcomp _enemykey)))))

(fn `UserConstructionScript`)